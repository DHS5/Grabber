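; BP_HookableObject is a mesh-based object that can be hooked, typed as Object among hookables.
; The OnHooked and OnUnhooked events set and clear an IsHooked flag, and CanBeHooked returns true only while that flag is false.
; GetAnchor returns the StaticMesh as the attachment point, and the construction script is empty.
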(event EventOnHooked
  (Variables|Hook|SetbIsHooked true))

(event EventOnUnhooked
  (Variables|Hook|SetbIsHooked false))

(fn ConstructionScript)

(fn CanbeHooked
  (return (not (Variables|Hook|GetbIsHooked))))

(fn GetAnchor
  (return (Variables|Default|GetStaticMesh)))

(fn GetType
  (return "HOOK_Object"))